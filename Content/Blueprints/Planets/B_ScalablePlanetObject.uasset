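; Planet actor that randomises its size, mass and glowing colour, and flashes when pulsed.
; Construction picks a random size that sets radius and sphere scale, then derives mass from sphere volume for the GameplayObjectComponent.
; A random hue, optionally tied to size, feeds a dynamic glow material.
; A bound pulse event multiplies the initial glow, which Tick eases back to normal.
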(event `self.ReceiveBeginPlay`
  (`|ExecutionSequence`
    (:`then_0`
      (set `self.InitialGlow` (`self.Glow`)))
    (:`then_1`
      (add `self.PulsePlanet` (delegate `PulsePlanet_Event`)))))

(event `self.ReceiveTick`
  (params (DeltaSeconds :type "Float (single-precision)"))
  (bind _returnvalue (`KismetMathLibrary.Lerp` (`self.Glow`) (`self.InitialGlow`) (* DeltaSeconds 4.0)))
  (set `self.Glow` _returnvalue)
  (`MaterialInstanceDynamic.SetScalarParameterValue` (`self.DynamicMaterialInstance`) "Glow" _returnvalue))

(event `PulsePlanet_Event`
  (set `self.Glow` (* (`self.InitialGlow`) 4.0)))

(fn `UserConstructionScript`
  (`|ExecutionSequence`
    (:`then_0`
      ;[1 1 1] Random size [0,1]
      (set `self.RandomSize` (`KismetMathLibrary.RandomFloatInRange` 0.0 1.0)))
    (:`then_1`
      (`|ExecutionSequence`
        (:`then_0`
          ;[1 1 1] Set radius from range
          (bind _output_get (set `self.Radius` (`KismetMathLibrary.MapRangeClamped` (`self.RandomSize`) 0.0 1.0 0.5 2.0)))
          (set `/Game/Blueprints/Gameplay/B_GameplayObjectComponent.Radius` _output_get (`self.GameplayObjectComponent`)))
        (:`then_1`
          ;[1 1 1] Set scale from radius
          (`SceneComponent.SetRelativeScale3D` (`self.Sphere`) (`KismetMathLibrary.Conv_DoubleToVector` (* (`self.Radius`) 2.0))))
        (:`then_2`
          ;[1 1 1] Set Mass
          (set `/Game/Blueprints/Gameplay/B_GameplayObjectComponent.Mass` (* (* (`KismetMathLibrary.MultiplyByPi` (`KismetMathLibrary.MultiplyMultiply_FloatFloat` (`self.Radius`) 3.0)) (/ 4.0 3.0)) (`self.Mass Per Volumetric Unit`)) (`self.GameplayObjectComponent`)))))
    (:`then_2`
      ;[1 1 1] Random HSV -> Linear RGB
      (set `self.Colour` (`KismetMathLibrary.HSVToRGBLinear` (make `LinearColor` (`KismetMathLibrary.MapRangeClamped` (`KismetMathLibrary.SelectFloat` (`self.RandomSize`) (`KismetMathLibrary.RandomFloatInRange` 0.0 1.0) (`self.BaseColourOnSize`)) 0.0 1.0 90.0 360.0) 1.0 (`KismetMathLibrary.RandomFloatInRange` 1.0 1.0) 1.0))))
    (:`then_3`
      ;[1 1 1] Create material and set colour/glow
      (bind _returnvalue (`PrimitiveComponent.CreateDynamicMaterialInstance` (`self.Sphere`) 0 "/Game/Materials/M_GlowPlanet.M_GlowPlanet" "None"))
      (`|ExecutionSequence`
        (:`then_0`
          (set `self.DynamicMaterialInstance` _returnvalue))
        (:`then_1`
          (`MaterialInstanceDynamic.SetVectorParameterValue` _returnvalue "EmissiveColour" (`self.Colour`)))
        (:`then_2`
          (`MaterialInstanceDynamic.SetScalarParameterValue` _returnvalue "Glow" (`self.Glow`)))))))