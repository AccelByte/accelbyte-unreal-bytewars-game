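; B_PlanetObject is a glowing planet actor whose sphere flashes brighter whenever a pulse event fires.
; The construction script creates a dynamic M_GlowPlanet material and applies the planet's colour, glow and scale.
; On BeginPlay it stores the base glow and binds to PulsePlanet, which jumps glow to a multiple of that base.
; Tick eases glow back to the base with a delta-time lerp and updates the material.
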(event `self.ReceiveBeginPlay`
  (`|ExecutionSequence`
    (:`then_0`
      (set `self.InitialGlow` (`self.Glow`)))
    (:`then_1`
      (add `self.PulsePlanet` (delegate `PulsePlanet_Event`)))))

(event `self.ReceiveTick`
  (params (DeltaSeconds :type "Float (single-precision)"))
  (bind _returnvalue (`KismetMathLibrary.Lerp` (`self.Glow`) (`self.InitialGlow`) (* DeltaSeconds 4.0)))
  (set `self.Glow` _returnvalue)
  (`MaterialInstanceDynamic.SetScalarParameterValue` (`self.DynamicMaterialInstance`) "Glow" _returnvalue))

(event `PulsePlanet_Event`
  (set `self.Glow` (* (`self.InitialGlow`) 4.0)))

(fn `UserConstructionScript`
  (bind _returnvalue (`PrimitiveComponent.CreateDynamicMaterialInstance` (`self.Sphere`) 0 "/Game/Materials/M_GlowPlanet.M_GlowPlanet" "None"))
  (set `self.Material` (`self.Material`))
  (`MaterialInstanceDynamic.SetVectorParameterValue` _returnvalue "EmissiveColour" (`self.Colour`))
  (`MaterialInstanceDynamic.SetScalarParameterValue` _returnvalue "Glow" (`self.Glow`))
  (`SceneComponent.SetRelativeScale3D` (`self.Sphere`) (`self.Scale`))
  (set `self.DynamicMaterialInstance` _returnvalue))