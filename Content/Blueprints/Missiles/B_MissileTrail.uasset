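; Missile trail actor Blueprint that drives the colour and opacity of a ribbon effect.
; An UpdateColour event pushes new colours to the MissileTrail component's ribbon parameter.
; Tick eases current alpha toward the wanted alpha, zeroes it below a tiny threshold and writes it to the ribbon's alpha scale.
; TriggerFadeOut, also run after a maximum lifetime, targets zero alpha, and IsFadedOut reports when it is reached.
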(event `self.ReceiveBeginPlay`
  (add `self.UpdateColour` (delegate `UpdateColour_Event`))
  (`KismetSystemLibrary.Delay` (`self.MaximumLifetime`))
  (`self.TriggerFadeOut`))

(event `UpdateColour_Event` :!signature `self.UpdateColour`
  (params (Colour :type "LinearColor Structure"))
  (bind _output_get (set `self.TrailColour` Colour))
  (`NiagaraComponent.SetVariableLinearColor` (`self.MissileTrail`) "RibbonColour" _output_get))

(event `self.ReceiveTick`
  (params (DeltaSeconds :type "Float (single-precision)"))
  (bind _returnvalue (`KismetMathLibrary.Lerp` (`self.CurrentAlpha`) (`self.WantedAlpha`) (* DeltaSeconds (`self.AlphaRate`))))
  (`|ExecutionSequence`
    (:`then_1`
      (`/Engine/EditorBlueprintResources/StandardMacros.CompareFloat` _returnvalue 1e-05
        (:`>`
          (set `self.CurrentAlpha` _returnvalue :!label _label))
        (:`==`
          (goto _label))
        (:`<`
          (bind _output_get (set `self.CurrentAlpha` 0.0))))
      (`NiagaraComponent.SetVariableFloat` (`self.MissileTrail`) "RibbonAlphaScale" _output_get))))

(fn `IsFadedOut`
  (returns (IsFadedOut :type Boolean))
  (return (not (> (`self.CurrentAlpha`) 0.0))))

(fn `TriggerFadeOut`
  (set `self.WantedAlpha` 0.0))

(fn `UserConstructionScript`)