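; Missile actor that flies under gravity from active game objects and accrues a score for its firing player.
; Each tick sums gravity, flags radius-overlap hits without physics collision, integrates velocity and aligns a separately spawned visual actor's parent to it.
; After one second, skimming near objects earns escalating bonuses, alongside time-alive points.
; Hits or timeout, preceded by expiry sparks, destroy it and notify the game mode, passing score on ship kills.
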(event `FireMissile_Event` :!signature `self.FireMissile`
  (params (InitialSpeed :type "Float (double-precision)") (PlayerController :type "/Game/Blueprints/Player/B_InGamePlayerController Object Reference"))
  ;[1 1 1] Set Initial Speed
  (set `self.PlayerController` PlayerController)
  (`self.SetInitialVelocity` InitialSpeed))

(event `self.ReceiveBeginPlay`
  (`|ExecutionSequence`
    (:`then_0`
      ;[1 1 1] Set Initial Speed
      (add `self.FireMissile` (delegate `FireMissile_Event`)))
    (:`then_1`
      ;[1 1 1] Attach Visual Actor
      (bind _returnvalue (`|SpawnActorFromClass` (`self.VisualActor`) (`KismetMathLibrary.MakeTransform` (0.0 0.0 0.0)) "Undefined" "OverrideRootScale" null null))
      (`self.K2_AttachToActor` _returnvalue self "None" "KeepRelative" "KeepRelative" "KeepRelative" true)
      (set `self.AttachedActor` _returnvalue))
    (:`then_2`
      ;[1 1 1] Get GameModeSettings
      (bind _asb_in_game_game_mode (cast `/Game/Blueprints/GameModes/B_InGameGameMode` (`GameplayStatics.GetGameMode`)))
      (bind _output_get (set `self.GameModeSettings` (`/Game/Blueprints/GameModes/B_InGameGameMode.GameModeSettings` _asb_in_game_game_mode)))
      (bind (_basescoreforkill _timescoreincrement _timescoredeltatime _skiminitialscore) (break `/Game/Blueprints/Gameplay/S_GameModeSettings` _output_get))
      (set `self.Score` (`KismetMathLibrary.Conv_IntToDouble` _basescoreforkill))
      (set `self.ScoreIncrement` (`KismetMathLibrary.Conv_IntToDouble` _skiminitialscore)))))

(event `self.ReceiveTick`
  (params (DeltaSeconds :type "Float (single-precision)"))
  (bind _gameplayobjectcomponent (`self.GameplayObjectComponent`))
  (bind _hitobject (`self.HitObject`))
  (bind _scoreincrement (`self.ScoreIncrement`))
  (bind (_basescoreforkill _timescoreincrement _timescoredeltatime _skiminitialscore _skimdeltaforincrementseconds _additionalskimscoremultiplier) (break `/Game/Blueprints/Gameplay/S_GameModeSettings` (`self.GameModeSettings`)))
  (bind (_basescoreforkill_2 _timescoreincrement_2 _timescoredeltatime_2) (break `/Game/Blueprints/Gameplay/S_GameModeSettings` (`self.GameModeSettings`)))
  (bind _returnvalue (+ (`self.TimeAlive`) DeltaSeconds))
  (bind _colour (`/Game/Blueprints/Gameplay/B_GameplayObjectComponent.Colour` _hitobject))
  (bind _returnvalue_2 (- (`KismetMathLibrary.FFloor` (/ _returnvalue _timescoredeltatime_2)) (`KismetMathLibrary.FFloor` (/ (`self.TimeAlive`) _timescoredeltatime_2))))
  (`|ExecutionSequence`
    (:`then_0`
      ;[1 1 1] Apply Gravity from all game objects in scene
      (bind _asb_in_game_game_state (cast `/Game/Blueprints/GameModes/B_InGameGameState` (`GameplayStatics.GetGameState`)))
      (set `self.GravityForce` (0.0 0.0 0.0))
      (for _array_element (`/Game/Blueprints/GameModes/B_InGameGameState.ActiveGameObjects` _asb_in_game_game_state)
        (if (`KismetSystemLibrary.IsValid` _array_element)
          (bind (_returnvalue_3 _returnvalue2) (`self.GetGravityForceToObject` _array_element _gameplayobjectcomponent))
          (set `self.GravityForce` (+ (`self.GravityForce`) _returnvalue2))
          (if (< (/ _returnvalue_3 100.0) (+ (`/Game/Blueprints/Gameplay/B_GameplayObjectComponent.Radius` _array_element) (`/Game/Blueprints/Gameplay/B_GameplayObjectComponent.Radius` _gameplayobjectcomponent)))
            (set `self.HitObject` _array_element)
            (set `self.KillActorThisFrame` true)))))
    (:`then_1`
      ;[1 1 1] Apply overall gravity force to change the velocity
      (set `self.Velocity` (+ (`self.Velocity`) (* (/ (`self.GravityForce`) (`/Game/Blueprints/Gameplay/B_GameplayObjectComponent.Mass` (`self.GameplayObjectComponent`))) (`GameplayStatics.GetWorldDeltaSeconds`)))))
    (:`then_2`
      ;[1 1 1] Update the objects position from the velocity
      (`self.K2_AddActorWorldOffset` (* DeltaSeconds (`self.Velocity`))))
    (:`then_3`
      ;[1 1 1] Align rotation with velocity direction
      (`self.AlignWithVelocityDirection` (`self.Velocity`)))
    (:`then_4`
      ;[1 1 1] Expiry (window before timeout destruction)
      (if (and (> (`self.GetGameTimeSinceCreation`) (- (`self.MaxTimeAlive`) (`self.ExpiryTime`))) (not (`self.Expiring`)))
        ;;[1 1 1] Deactivate constant thrust sparks, switch to intermittent expiring sparks
        (bind _asb_neon_object_missile (cast `/Game/Blueprints/Missiles/B_NeonObject_Missile` (`self.AttachedActor`)))
        (`|ExecutionSequence`
          (:`then_0`
            (`ActorComponent.Deactivate` (`/Game/Blueprints/Missiles/B_NeonObject_Missile.ThrustSparks` _asb_neon_object_missile)))
          (:`then_1`
            (`ActorComponent.Activate` (`/Game/Blueprints/Missiles/B_NeonObject_Missile.ExpiringSparks` _asb_neon_object_missile) false))
          (:`then_2`
            (set `self.Expiring` true)))))
    (:`then_5`
      ;[1 1 1] Timeout Destruct
      (if (> (`self.GetGameTimeSinceCreation`) (`self.MaxTimeAlive`))
        (set `self.KillActorThisFrame` true)))
    (:`then_6`
      (bind _asb_in_game_game_mode (cast `/Game/Blueprints/GameModes/B_InGameGameMode` (`GameplayStatics.GetGameMode`)))
      (bind _asb_in_game_game_state_2 (cast `/Game/Blueprints/GameModes/B_InGameGameState` (`GameplayStatics.GetGameState`)))
      (if (> (`self.GetGameTimeSinceCreation`) 1.0)
        (`|ExecutionSequence`
          (:`then_0`
            (bind (_score _output_get _isskimming) (`self.IsSkimmingPlanet` DeltaSeconds (`/Game/Blueprints/GameModes/B_InGameGameState.ActiveGameObjects` _asb_in_game_game_state_2)))
            (if _isskimming
              (set `self.TimeSkimmingPlanet` (+ (`self.TimeSkimmingPlanet`) DeltaSeconds))
              (set `self.TimeSkimmingPlanetReward` (+ (`self.TimeSkimmingPlanetReward`) DeltaSeconds))
              (else
                (set `self.TimeSkimmingPlanet` 0.0)
                (set `self.TimeSkimmingPlanetReward` 0.0))))
          (:`then_1`
            (if (> (`self.TimeSkimmingPlanetReward`) _skimdeltaforincrementseconds)
              (`|ExecutionSequence`
                (:`then_0`
                  (set `self.TimeSkimmingPlanetReward` 0.0)
                  (bind _output_get_2 (set `self.Score` (+ (`self.Score`) _scoreincrement)))
                  (`/Game/Blueprints/GameModes/B_InGameGameMode.OnMissileScoreUpdated` _asb_in_game_game_mode (`KismetMathLibrary.FTrunc` _output_get_2) (`KismetMathLibrary.FTrunc` _scoreincrement) (`self.GameplayObjectComponent`) (`self.PlayerController`)))
                (:`then_1`
                  (set `self.ScoreIncrement` (* (`self.ScoreIncrement`) _additionalskimscoremultiplier))))))
          (:`then_2`
            (`|ExecutionSequence`
              (:`then_0`
                (if (> _returnvalue_2 0)
                  (bind _output_get_3 (set `self.Score` (+ (* _returnvalue_2 _timescoreincrement_2) (`self.Score`))))))
              (:`then_1`
                (set `self.TimeAlive` _returnvalue)))))))
    (:`then_7`
      ;[1 1 1] On Destroy Object
      (if (`self.KillActorThisFrame`)
        (`self.K2_DestroyActor` (`self.AttachedActor`))
        (`self.K2_DestroyActor`)
        (bind _asb_in_game_game_mode_2 (cast `/Game/Blueprints/GameModes/B_InGameGameMode` (`GameplayStatics.GetGameMode`)))
        (if (`KismetSystemLibrary.IsValid` _hitobject)
          (`/Game/Blueprints/GameModes/B_InGameGameMode.OnMissileDestroyed` _asb_in_game_game_mode_2 (`self.K2_GetActorLocation`) _colour _hitobject (`self.Velocity`) (`self.MissileColour`))
          (if (`|EnumEquality` (`/Game/Blueprints/Gameplay/B_GameplayObjectComponent.GameplayObjectType` _hitobject) "NewEnumerator0")
            (`/Game/Blueprints/GameModes/B_InGameGameMode.OnShipDestroyed` _asb_in_game_game_mode_2 _hitobject (`self.GameplayObjectComponent`) _colour (`self.Score`) (`self.PlayerController`))
            (set `self.HitObject` null))
          (else
            ;[1 1 1] If no object was hit, treat this as an expiry
            (`/Game/Blueprints/GameModes/B_InGameGameMode.CreateExpiredMissileExplosion` _asb_in_game_game_mode_2 (`self.K2_GetActorLocation`) (`self.MissileColour`))))))))

(fn `IsSkimmingPlanet`
  (params (A :type "Float (double-precision)") (Array :type "Array of /Game/Blueprints/Gameplay/B_GameplayObjectComponent Object Reference"))
  (returns (Score :type "Float (double-precision)") (Output_Get :type "Float (double-precision)") (IsSkimming :type Boolean))
  (bind _gameplayobjectcomponent (`self.GameplayObjectComponent`))
  (for _array_element Array
    (if (`KismetSystemLibrary.IsValid` _array_element)
      (if (`KismetSystemLibrary.IsValid` _gameplayobjectcomponent)
        (if (< (`self.GetSurfaceDistanceBetweenObjects` _array_element _gameplayobjectcomponent) 100.0)
          (return 0.0 0.0 true)))))
  (return 0.0 0.0 false))

(fn `UserConstructionScript`)