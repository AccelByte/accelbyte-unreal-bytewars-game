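; Player pawn for a neon ship that fires one missile at a time at a speed set by power level.
; BeginPlay attaches a spawned ship visual and binds input, fire and colour events, passing player colour to ship, missile and trail.
; Firing increments the PlayerState shot count, fades old trails and spawns a sound actor.
; Tick briefly shows a projected power bar after input and removes faded trails and finished sounds.
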(event `OnPlayerInputThisFrame_Event`
  (set `self.ShowPowerLevelUITimer` 1.0))

(event `UpdateColour_Event` :!signature `self.UpdateColour`
  (params (Colour :type "LinearColor Structure"))
  (set `/Game/Blueprints/Gameplay/B_GameplayObjectComponent.Colour` Colour (`self.GameplayObjectComponent`))
  (`/Game/Blueprints/Ships/B_NeonObject.UpdateColour` (stale `self.ReceiveBeginPlay` _asb_neon_object) (`/Game/Blueprints/Gameplay/B_GameplayObjectComponent.Colour` (`self.GameplayObjectComponent`)) :!label _label))

(event `self.ReceiveBeginPlay`
  (`|ExecutionSequence`
    (:`then_1`
      (add `self.OnPlayerInputThisFrame` (delegate `OnPlayerInputThisFrame_Event`)))
    (:`then_2`
      (add `self.FireMissile` (delegate `FireMissile_Event`)))
    (:`then_3`
      (bind _returnvalue (`|SpawnActorFromClass` (`self.NeonShipActor`) (`KismetMathLibrary.MakeTransform` (0.0 0.0 0.0)) "Undefined" "OverrideRootScale" null null))
      (bind _asb_neon_object (cast `/Game/Blueprints/Ships/B_NeonObject` _returnvalue))
      (`self.K2_AttachToActor` _returnvalue self "None" "KeepRelative" "KeepRelative" "KeepRelative" true)
      (goto _label))
    (:`then_4`
      (add `self.UpdateColour` (delegate `UpdateColour_Event`)))))

(event `FireMissile_Event`
  (bind _rotation (.rotation (`self.GetTransform`)))
  (bind _colour (`/Game/Blueprints/Gameplay/B_GameplayObjectComponent.Colour` (`self.GameplayObjectComponent`)))
  (bind _returnvalue (`KismetMathLibrary.MakeTransform` (+ (* (`KismetMathLibrary.GetRightVector` _rotation) 90.0) (.location (`self.GetTransform`))) _rotation))
  (if (not (`KismetSystemLibrary.IsValid` (`self.FiredMissile`)))
    (`|ExecutionSequence`
      (:`then_0`
        (bind _returnvalue_2 (`|SpawnActorFromClass` (`self.MissileActor`) _returnvalue "Undefined" "OverrideRootScale" null null))
        (set `self.FiredMissile` _returnvalue_2)
        (bind _asb_missile (cast `/Game/Blueprints/Missiles/B_Missile` _returnvalue_2))
        (set `/Game/Blueprints/Missiles/B_Missile.MissileColour` _colour _asb_missile)
        (bind _asb_neon_object (cast `/Game/Blueprints/Ships/B_NeonObject` (`/Game/Blueprints/Missiles/B_Missile.AttachedActor` _asb_missile)))
        (`/Game/Blueprints/Ships/B_NeonObject.UpdateColour` _asb_neon_object _colour)
        (bind _asin_game_player_controller (cast `/Game/Blueprints/Player/B_InGamePlayerController` (`self.GetController`)))
        (`/Game/Blueprints/Missiles/B_Missile.FireMissile` _asb_missile (`KismetMathLibrary.MapRangeClamped` (`self.FirePowerLevel`) 0.0 1.0 (`self.MinMissileSpeed`) (`self.MaxMissileSpeed`)) _asin_game_player_controller)
        (set `self.ShowPowerLevelUITimer` 0.0))
      (:`then_1`
        (bind _returnvalue_3 (`|SpawnActorFromClass` "/Game/Blueprints/Ships/B_FireMissile.B_FireMissile_C" _returnvalue "Undefined" "OverrideRootScale" null null))
        (`KismetArrayLibrary.Array_Add` (`self.FiredMissiles`) _returnvalue_3))
      (:`then_2`
        (bind _asin_game_player_state (cast `/Game/Blueprints/Player/B_InGamePlayerState` (`self.PlayerState`)))
        (set `/Game/Blueprints/Player/B_InGamePlayerState.NumMissilesFired` (+ (`/Game/Blueprints/Player/B_InGamePlayerState.NumMissilesFired` _asin_game_player_state) 1) _asin_game_player_state))
      (:`then_3`
        ;[1 1 1] Start fade out on existing trails when new missile is fired
        (for _array_element (`self.MissileTrail`)
          (`/Game/Blueprints/Missiles/B_MissileTrail.TriggerFadeOut` _array_element))
        ;[1 1 1] Create missile trail, piggy back missile  and set colour to player
        (bind _returnvalue_4 (`|SpawnActorFromClass` "/Game/Blueprints/Missiles/B_MissileTrail.B_MissileTrail_C" _returnvalue "Undefined" "OverrideRootScale" null null))
        (`KismetArrayLibrary.Array_Add` (`self.MissileTrail`) _returnvalue_4)
        (`self.K2_AttachToActor` _returnvalue_4 (`self.FiredMissile`) "None" "SnapToTarget" "SnapToTarget" "KeepRelative" true)
        (`/Game/Blueprints/Missiles/B_MissileTrail.UpdateColour` _returnvalue_4 (`/Game/Blueprints/Gameplay/B_GameplayObjectComponent.Colour` (`self.GameplayObjectComponent`)))))))

(event `self.ReceiveTick`
  (params (DeltaSeconds :type "Float (single-precision)"))
  (bind _showpowerleveluitimer (`self.ShowPowerLevelUITimer`))
  (bind _missiletrail (`self.MissileTrail`))
  (`|ExecutionSequence`
    (:`then_0`
      (bind _asin_game_player_state (cast `/Game/Blueprints/Player/B_InGamePlayerState` (`self.PlayerState`)))
      (if (> _showpowerleveluitimer 0.0)
        (set `self.ShowPowerLevelUITimer` (`KismetMathLibrary.FClamp` (- _showpowerleveluitimer (`GameplayStatics.GetWorldDeltaSeconds`)) 0.0 100.0))
        (bind _powerbarui (`/Game/Blueprints/Player/B_InGamePlayerState.PowerBarUI` _asin_game_player_state))
        (`Widget.SetVisibility` _powerbarui "Visible")
        (cast `/Game/Blueprints/Player/B_InGamePlayerController` (`self.GetController`))
        (`UserWidget.SetPositionInViewport` _powerbarui (`PlayerController.ProjectWorldLocationToScreen` (`GameplayStatics.GetPlayerController` 0) (+ (`self.K2_GetActorLocation`) (-150.0 0.0 0.0)) false) true)
        (else
          (`Widget.SetVisibility` _powerbarui "Hidden"))))
    (:`then_1`
      ;[1 1 1] Remove faded out trails
      (bind (_arrayindex _arrayelement) (`/Engine/EditorBlueprintResources/StandardMacros.ReverseForEachLoop` _missiletrail)
        (:`LoopBody`
          (bind _isfadedout (`/Game/Blueprints/Missiles/B_MissileTrail.IsFadedOut` _arrayelement))
          (if _isfadedout
            (`self.K2_DestroyActor` _arrayelement)
            (`KismetArrayLibrary.Array_Remove` _missiletrail _arrayindex)))))
    (:`then_2`
      ;[1 1 1] Remove Fired Missiles when audio has finished
      (bind (_arrayindex_2 _arrayelement_2) (`/Engine/EditorBlueprintResources/StandardMacros.ReverseForEachLoop` (`self.FiredMissiles`))
        (:`LoopBody`
          (bind _finished_playing (`/Game/Blueprints/Ships/B_FireMissile.GetHasFinishedPlaying` _arrayelement_2))
          (if _finished_playing
            (`self.K2_DestroyActor` _arrayelement_2)
            (`KismetArrayLibrary.Array_Remove` (`self.FiredMissiles`) _arrayindex_2)))))))

(fn `UserConstructionScript`)