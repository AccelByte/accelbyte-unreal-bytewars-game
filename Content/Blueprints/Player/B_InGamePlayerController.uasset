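; In-game player controller that turns player input into actions on the controlled B_PlayerPawn ship.
; RotateShip yaws the pawn by a frame-time-scaled, inverted axis value, while FireMissile tells the pawn to fire.
; AdjustFirePower changes the pawn's FirePowerLevel over time, clamped between zero and one.
; Only the fire-power axis notifies the pawn of input each frame, through a helper that ignores zero values.
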(event `InputAxis|AdjustFirePower`
  (params (AxisValue :type "Float (single-precision)"))
  (bind _returnvalue (`self.K2_GetPawn`))
  (`self.InformPawnPlayerInputThisFrame` AxisValue _returnvalue)
  (bind _asplayer_pawn (cast `/Game/Blueprints/Player/B_PlayerPawn` _returnvalue))
  (set `/Game/Blueprints/Player/B_PlayerPawn.FirePowerLevel` (`KismetMathLibrary.FClamp` (+ (`/Game/Blueprints/Player/B_PlayerPawn.FirePowerLevel` _asplayer_pawn) (* (`GameplayStatics.GetWorldDeltaSeconds`) (`self.FirePowerChangeSpeed`) AxisValue))) _asplayer_pawn))

(event `InputAction|FireMissile`
  (params (Key :type "Key Structure"))
  (:`Pressed`
    (bind _asplayer_pawn (cast `/Game/Blueprints/Player/B_PlayerPawn` (`self.K2_GetPawn`)))
    (`/Game/Blueprints/Player/B_PlayerPawn.FireMissile` _asplayer_pawn)))

(event `self.ReceiveBeginPlay`
  (`self.EnableInput` self))

(event `self.ReceiveTick`
  (params (DeltaSeconds :type "Float (single-precision)")))

(event `InputAxis|RotateShip`
  (params (AxisValue :type "Float (single-precision)"))
  (bind _returnvalue (`self.K2_GetPawn`))
  (if (`KismetSystemLibrary.IsValid` _returnvalue)
    (`self.K2_AddActorWorldRotation` _returnvalue (* (`KismetMathLibrary.MakeRotator` 0.0 0.0 (* (`GameplayStatics.GetWorldDeltaSeconds`) (`self.RotateSpeed`) AxisValue)) -1.0) false false)))

(fn `InformPawnPlayerInputThisFrame`
  (params (A :type "Float (double-precision)") (PlayerPawn :type "Object Object Reference"))
  (if (!= A 0.0)
    (bind _asplayer_pawn (cast `/Game/Blueprints/Player/B_PlayerPawn` PlayerPawn))
    (`/Game/Blueprints/Player/B_PlayerPawn.OnPlayerInputThisFrame` _asplayer_pawn)
    (return)))

(fn `UserConstructionScript`)