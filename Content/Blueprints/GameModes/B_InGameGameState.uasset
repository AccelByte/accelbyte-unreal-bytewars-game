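; B_InGameGameState is the in-game GameState Blueprint that provides player-survival queries over its Teams and their Players.
; GetNumPlayersAlive loops through every team's players and, despite its name, counts those whose NumLivesLeft equals zero.
; GetLastPlayerAlive returns the first player found with lives remaining, without checking that it is the only one.
; The event graph and construction script hold no logic.
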(fn `GetLastPlayerAlive`
  (returns (PlayerState :type "/Game/Blueprints/Player/B_InGamePlayerState Object Reference"))
  (for _array_element (`self.Teams`)
    (for _array_element_2 (`.Players_7_9F04DC0A4DF8734084BEAE9A518C718F` (break `/Game/Blueprints/Gameplay/S_Team` _array_element))
      (if (> (`/Game/Blueprints/Player/B_InGamePlayerState.NumLivesLeft` _array_element_2) 0)
        (return _array_element_2))))
  (return null))

(fn `GetNumPlayersAlive`
  (returns (NumPlayersStillAlive :type Integer))
  (locals (NumPlayersAlive :type Integer))
  (for _array_element (`self.Teams`)
    (for _array_element_2 (`.Players_7_9F04DC0A4DF8734084BEAE9A518C718F` (break `/Game/Blueprints/Gameplay/S_Team` _array_element))
      (if (== (`/Game/Blueprints/Player/B_InGamePlayerState.NumLivesLeft` _array_element_2) 0)
        (bind _result (`/Engine/EditorBlueprintResources/StandardMacros.IncrementInt` (`local.NumPlayersAlive`))
          (:`  `
            (set `local.NumPlayersAlive` _result))))))
  (return (`local.NumPlayersAlive`)))

(fn `UserConstructionScript`)