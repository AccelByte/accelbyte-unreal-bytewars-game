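; In-game orthographic camera that zooms to keep gameplay objects in frame and pulses a post-process intensity.
; Each tick it scans all actors for B_GameplayObjectComponent, using absolute location, radius and a buffer to size a view symmetric about the world origin.
; Ortho width respects aspect ratio and stays between the starting extents and a multiple of them.
; PulseBackgroundEvent spikes the intensity, which eases back to baseline every tick.
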(event `self.ReceiveBeginPlay`
  (bind _cameracomponent (`self.CameraComponent`))
  (bind _orthowidth (`CameraComponent.OrthoWidth` _cameracomponent))
  (`|ExecutionSequence`
    (:`then_0`
      ;[0 0 0] Set min and max extents
      (bind _output_get (set `self.MinExtents` (`KismetMathLibrary.MakeVector` _orthowidth (/ _orthowidth (`CameraComponent.AspectRatio` _cameracomponent)))))
      (bind _output_get_2 (set `self.FurthestPositionToFrame` _output_get))
      (set `self.MaxExtents` (* _output_get_2 2.5)))
    (:`then_1`
      ;[0 0 0] bind pulse background event
      (add `self.PulseBackgroundEvent` (delegate `PulseBackgroundEvent_Event`)))))

(event `PulseBackgroundEvent_Event`
  ;[0 0 0] bind pulse background event
  (set `self.PulseTarget` 3.5))

(event `self.ReceiveTick`
  (params (DeltaSeconds :type "Float (single-precision)"))
  (`|ExecutionSequence`
    (:`then_0`
      (`self.AdjustCameraWidth`))
    (:`then_1`
      ;[0 0 0] Set pulse target
      (set `self.PulseTarget` (`KismetMathLibrary.Lerp` (`self.PulseTarget`) 0.6 (* DeltaSeconds 4.0))))
    (:`then_2`
      ;[0 0 0] Set post process settings
      (setmembers `PostProcessSettings` :`StructRef` (`CameraComponent.PostProcessSettings` (`self.CameraComponent`)) :`BloomIntensity` (`self.PulseTarget`) :`AutoExposureBiasCurve` null))))

(fn `AdjustCameraWidth`
  (bind _outactors (`GameplayStatics.GetAllActorsOfClass` "/Script/Engine.Actor"))
  (set `self.FurthestPositionToFrame` (`self.MinExtents`))
  ;[0 0 0] Iterate through all the actors available and set the furthest to frame
  (for _array_element _outactors
    (bind _returnvalue (`self.GetComponentByClass` _array_element "/Game/Blueprints/Gameplay/B_GameplayObjectComponent.B_GameplayObjectComponent_C"))
    (if (`KismetSystemLibrary.IsValid` _returnvalue)
      (set `self.FurthestPositionToFrame` (`KismetMathLibrary.Vector_ComponentMax` (+ (* (+ (`KismetMathLibrary.Vector_GetAbs` (`self.K2_GetActorLocation` _array_element)) (* (`/Game/Blueprints/Gameplay/B_GameplayObjectComponent.Radius` _returnvalue) 100.0)) 2.0) (`self.BufferWidth`)) (`self.FurthestPositionToFrame`)))))
  ;[0 0 0] Set orthographic width on iteration completed
  (`CameraComponent.SetOrthoWidth` (`self.CameraComponent`) (`KismetMathLibrary.FMax` (.x (`KismetMathLibrary.Vector_ComponentMin` (`self.FurthestPositionToFrame`) (`self.MaxExtents`))) (* (.y (`KismetMathLibrary.Vector_ComponentMin` (`self.FurthestPositionToFrame`) (`self.MaxExtents`))) (`CameraComponent.AspectRatio` (`self.CameraComponent`))))))

(fn `UserConstructionScript`)