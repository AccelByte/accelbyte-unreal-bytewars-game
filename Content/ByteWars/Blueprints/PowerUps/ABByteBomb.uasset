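; ABByteBomb is the Byte Bomb power-up Blueprint that, when detonated, shakes the camera and wipes out enemy missiles.
; On InitiateExplosion it passes the owning pawn and B_CameraShake to ServerShakeCamera.
; It then resolves the owner's team through pawn, controller and player state, and passes that TeamId to ServerDestroyAllEnemyMissiles.
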(event `self.InitiateExplosion`
  (bind _returnvalue (`self.GetOwner`))
  (bind _aspawn (cast `Pawn` _returnvalue))
  (`self.Server_ShakeCamera` _aspawn "/Game/ByteWars/Blueprints/Cameras/B_CameraShake.B_CameraShake_C")
  (bind _asaccel_byte_wars_player_pawn (cast `AccelByteWarsPlayerPawn` _returnvalue))
  (bind _asaccel_byte_wars_player_controller (cast `AccelByteWarsPlayerController` (`Pawn.GetController` _asaccel_byte_wars_player_pawn)))
  (bind _playerstate (`Controller.PlayerState` _asaccel_byte_wars_player_controller))
  (`/Engine/EditorBlueprintResources/StandardMacros.IsValid` _playerstate
    (:`Is Valid`
      (bind _asaccel_byte_wars_player_state (cast `AccelByteWarsPlayerState` _playerstate))
      (`self.Server_DestroyAllEnemyMissiles` _aspawn (`AccelByteWarsPlayerState.TeamId` _asaccel_byte_wars_player_state)))))

(fn `UserConstructionScript`)