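; Main menu GameState for ByteWars that refreshes the join screen's player entries when team data is notified.
; OnNotifyTeams finds the Menu stack in the GameInstance's base UI and, if the active widget is W_Join, calls its multiplayer player-entry generation.
; TriggerUpdateClientUI runs the same refresh, skipping it on dedicated servers.
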(event `self.OnNotify_Teams`
  ;[0 0 0] OnNotify Teams data and trigger update UI: Get currently active widget from widget stack
  (bind _asaccel_byte_wars_game_instance (cast `AccelByteWarsGameInstance` (`GameplayStatics.GetGameInstance`) :!label _label))
  (bind _asaccel_byte_wars_base_ui (cast `AccelByteWarsBaseUI` (`AccelByteWarsGameInstance.BaseUIWidget` _asaccel_byte_wars_game_instance)))
  (bind (_value _returnvalue) (`BlueprintMapLibrary.Map_Find` (`AccelByteWarsBaseUI.Stacks` _asaccel_byte_wars_base_ui) "Menu"))
  (if _returnvalue
    (bind _returnvalue_2 (`CommonActivatableWidgetContainerBase.GetActiveWidget` _value))
    (`/Engine/EditorBlueprintResources/StandardMacros.IsValid` _returnvalue_2
      (:`Is Valid`
        (bind _asw_join (cast `/Game/ByteWars/UI/MainMenu/Multiplayer/W_Join` _returnvalue_2))
        (`/Game/ByteWars/UI/MainMenu/Multiplayer/W_Join.Generate Player Entries Mulriplayer Checked` _asw_join)))))

(event `Trigger Update Client UI`
  ;[0 0 0] OnNotify Teams data and trigger update UI: Get currently active widget from widget stack
  (if (not (`KismetSystemLibrary.IsDedicatedServer`))
    (goto _label)))

(fn `UserConstructionScript`)