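; Main menu game mode for ByteWars that handles lobby readiness and travel into a match.
; On BeginPlay it removes local players other than controller ID 0, and on logout it clears the exiting player's ready flag.
; The readiness check refreshes client UI, then server-travels to GalaxyWorld once ready team members, resolved to player states by unique net ID, reach the registered player count.
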(event `self.ReceiveBeginPlay`
  ;[0 0 0] BeginPlay sequences: remove local players that is not the first local player
  (for _array_element (`GameStateBase.PlayerArray` (`GameplayStatics.GetGameState`))
    (bind _returnvalue (`PlayerState.GetPlayerController` _array_element))
    (if (`Controller.IsLocalPlayerController` _returnvalue)
      (if (not (== (`GameplayStatics.GetPlayerControllerID` _returnvalue) 0))
        (`GameplayStatics.RemovePlayer` _returnvalue)))))

(event `self.K2_OnLogout`
  (params (ExitingController :type "Controller Object Reference"))
  ;[0 0 0] OnLogout: set player's readyness to false
  (bind _asb_main_menu_player_state (cast `/Game/ByteWars/Blueprints/Player/B_MainMenuPlayerState` (`Controller.PlayerState` ExitingController)))
  (set `/Game/ByteWars/Blueprints/Player/B_MainMenuPlayerState.bIsReady` false _asb_main_menu_player_state))

(fn `IsEveryoneReady`
  (returns (bIsReady :type Boolean))
  (locals (CurrentlyReady :type Integer) (GameState :type "AccelByteWarsGameStateBase Object Reference"))
  (bind _currentlyready (`local.CurrentlyReady`))
  (bind _asaccel_byte_wars_game_state_base (cast `AccelByteWarsGameStateBase` (`GameplayStatics.GetGameState`)))
  (set `local.GameState` _asaccel_byte_wars_game_state_base)
  (`|ExecutionSequence`
    (:`then_0`
      ;[0 0 0] Get how many players is currently ready
      (for _array_element (`AccelByteWarsGameStateBase.Teams` (`local.GameState`))
        (for _array_element_2 (`.TeamMembers` (break `GameplayTeamData` _array_element))
          (bind _returnvalue (`GameplayStatics.GetPlayerStateFromUniqueNetId` (`.UniqueNetId` (break `GameplayPlayerData` _array_element_2))))
          (`/Engine/EditorBlueprintResources/StandardMacros.IsValid` _returnvalue
            (:`Is Valid`
              (bind _asb_main_menu_player_state (cast `/Game/ByteWars/Blueprints/Player/B_MainMenuPlayerState` _returnvalue))
              (if (`/Game/ByteWars/Blueprints/Player/B_MainMenuPlayerState.bIsReady` _asb_main_menu_player_state)
                (`/Engine/EditorBlueprintResources/StandardMacros.IncrementInt` (`local.CurrentlyReady`))))))))
    (:`then_1`
      ;[0 0 0] return
      (`KismetSystemLibrary.PrintString` (`KismetStringLibrary.Conv_IntToString` _currentlyready))
      (return (>= _currentlyready (`AccelByteWarsGameStateBase.GetRegisteredPlayersNum` (`local.GameState`)))))))

(fn `Server Travel to Game if Everyone Ready`
  (bind _asb_main_menu_game_state (cast `/Game/ByteWars/Blueprints/GameModes/B_MainMenuGameState` (`GameplayStatics.GetGameState`)))
  (`/Game/ByteWars/Blueprints/GameModes/B_MainMenuGameState.Trigger Update Client UI` _asb_main_menu_game_state)
  (if (`self.IsEveryoneReady`)
    (`self.TriggerServerTravel` "/Game/ByteWars/Maps/GalaxyWorld/GalaxyWorld.GalaxyWorld")))

(fn `UserConstructionScript`)