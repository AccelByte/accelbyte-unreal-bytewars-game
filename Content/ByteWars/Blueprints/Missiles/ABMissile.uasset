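; ABMissile is the missile Blueprint for ByteWars, handling its procedural mesh appearance and score popup feedback.
; Its construction script sets up the procedural mesh and tints it with the missile's color.
; A SpawnScorePopupHud event shows a score popup at the missile's location in that color through player 0's B_HUD, skipped on dedicated servers.
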(event `self.SpawnScorePopupHud`
  (params (InScore :type Integer))
  (bind _returnvalue (`GameplayStatics.GetPlayerControllerFromID` 0))
  (bind _returnvalue_2 (`PlayerController.GetHUD` _returnvalue))
  ;[0 0 0] Spawn ScorePopup HUD
  (if (not (`KismetSystemLibrary.IsDedicatedServer`))
    (`/Engine/EditorBlueprintResources/StandardMacros.IsValid` _returnvalue
      (:`Is Valid`
        (`/Engine/EditorBlueprintResources/StandardMacros.IsValid` _returnvalue_2
          (:`Is Valid`
            (bind _asb_hud (cast `/Game/ByteWars/UI/HUD/B_HUD` _returnvalue_2))
            (`/Game/ByteWars/UI/HUD/W_HUD_ScorePopup.SpawnScore` (`/Game/ByteWars/UI/HUD/B_HUD.ScorePopupUI` _asb_hud) (`self.K2_GetActorLocation`) (`self.Color`) InScore)))))))

(fn `UserConstructionScript`
  (bind _accelbytewarsproceduralmesh (`self.AccelByteWarsProceduralMesh`))
  (`AccelByteWarsProceduralMeshComponent.MeshSetup` _accelbytewarsproceduralmesh)
  (`AccelByteWarsProceduralMeshComponent.UpdateColor` _accelbytewarsproceduralmesh (`self.Color`)))