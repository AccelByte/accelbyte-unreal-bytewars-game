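; B_MissileTrail is the actor that renders a missile's coloured Niagara ribbon trail and fades it out.
; Trail colour is set in the construction script and reapplied by its RepNotify.
; TriggerFadeOut, also fired after a maximum lifetime, zeroes the target alpha, which Tick lerps toward and writes to the ribbon, snapping tiny values to zero.
; IsFadedOut reports completion, and the actor destroys itself when its owner is destroyed.
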(event `self.ReceiveBeginPlay`
  (bind _returnvalue (`self.GetOwner`))
  ;[0 0 0] BeginPlay sequences
  (`|ExecutionSequence`
    (:`then_0`
      ;;[0 0 0] Trigger fade out on delay
      (`KismetSystemLibrary.Delay` (`self.MaximumLifetime`))
      (`self.TriggerFadeOut`))
    (:`then_1`
      ;;[0 0 0] Destroy this actor on owner destroyed
      (`/Engine/EditorBlueprintResources/StandardMacros.IsValid` _returnvalue
        (:`Is Valid`
          (add `self.OnDestroyed` _returnvalue (delegate `OnDestroyed_Event`)))))))

(event `OnDestroyed_Event` :!signature `self.OnDestroyed`
  (params (DestroyedActor :type "Actor Object Reference"))
  ;[0 0 0] BeginPlay sequences
  ;;[0 0 0] Destroy this actor on owner destroyed
  (`self.K2_DestroyActor`))

(event `self.ReceiveTick`
  (params (DeltaSeconds :type "Float (single-precision)"))
  (bind _returnvalue (`KismetMathLibrary.Lerp` (`self.CurrentAlpha`) (`self.WantedAlpha`) (* DeltaSeconds (`self.AlphaRate`))))
  ;[0 0 0] Tick sequences
  (`/Engine/EditorBlueprintResources/StandardMacros.CompareFloat` _returnvalue 1e-05
    (:`>`
      (set `self.CurrentAlpha` _returnvalue :!label _label))
    (:`==`
      (goto _label))
    (:`<`
      (bind _output_get (set `self.CurrentAlpha` 0.0))))
  (`NiagaraComponent.SetVariableFloat` (`self.MissileTrail`) "RibbonAlphaScale" _output_get))

(fn `IsFadedOut`
  (returns (IsFadedOut :type Boolean))
  (return (not (> (`self.CurrentAlpha`) 0.0))))

(fn `OnRep_TrailColour`
  (`NiagaraComponent.SetVariableLinearColor` (`self.MissileTrail`) "RibbonColour" (`self.TrailColour`)))

(fn `TriggerFadeOut`
  (set `self.WantedAlpha` 0.0))

(fn `UserConstructionScript`
  (`NiagaraComponent.SetVariableLinearColor` (`self.MissileTrail`) "RibbonColour" (`self.TrailColour`)))