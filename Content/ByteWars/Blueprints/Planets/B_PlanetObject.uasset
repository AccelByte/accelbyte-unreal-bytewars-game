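; Planet actor for Byte Wars that renders a coloured, glowing sphere which pulses in brightness on an event, likely a hit.
; The construction script creates a dynamic M_GlowPlanet material, applies the colour and scale, and takes the default glow from a global material parameter collection.
; The pulse event multiplies the initial glow on everything except dedicated servers, and Tick eases it back while updating the material.
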(event `PulsePlanet_Event`
  ;[0 0 0] Event: set glow
  (if (not (`KismetSystemLibrary.IsDedicatedServer`))
    (set `self.Glow` (* (`self.InitialGlow`) (`self.HitPulseMultiplier`)))))

(event `self.ReceiveBeginPlay`
  ;[0 0 0] BeginPlay sequences: set initial glow
  (set `self.InitialGlow` (`self.Glow`)))

(event `self.ReceiveTick`
  (params (DeltaSeconds :type "Float (single-precision)"))
  ;[0 0 0] Tick sequences: show glow
  (bind _output_get (set `self.Glow` (`KismetMathLibrary.Lerp` (`self.Glow`) (`self.InitialGlow`) (* DeltaSeconds 4.0))))
  (`MaterialInstanceDynamic.SetScalarParameterValue` (`self.DynamicMaterialInstance`) "Glow" _output_get))

(fn `UserConstructionScript`
  (bind _returnvalue (`PrimitiveComponent.CreateDynamicMaterialInstance` (`self.Sphere`) 0 "/Game/ByteWars/Materials/M_GlowPlanet.M_GlowPlanet" "None"))
  (set `self.Material` (`self.Material`))
  (`MaterialInstanceDynamic.SetVectorParameterValue` _returnvalue "EmissiveColour" (`self.Colour`))
  (set `self.Glow` (`.ReturnValue` (`MaterialParameterCollection.GetScalarParameterDefaultValue` (`AccelByteWarsBlueprintFunctionLibrary.GetGlobalMaterialParameterCollection`) "PlanetGlow")))
  (`MaterialInstanceDynamic.SetScalarParameterValue` _returnvalue "Glow" (`self.Glow`))
  (`SceneComponent.SetRelativeScale3D` (`self.Sphere`) (`self.Scale`))
  (set `self.DynamicMaterialInstance` _returnvalue))