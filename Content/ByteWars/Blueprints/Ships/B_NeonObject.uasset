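; B_NeonObject is a Byte Wars ship-related actor that draws a glowing neon outline as a procedural mesh.
; The construction script mirrors OutlineVertices across local X to complete the shape, pairs each vertex with one inset toward the origin, and builds a triangle strip.
; The radial inset yields uneven stroke width, flagged as a TODO.
; A dynamic M_NeonGlow material takes colour and glow, and a bound event updates the colour at runtime.
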(event `self.ReceiveBeginPlay`
  (`|ExecutionSequence`
    (:`then_0`
      (add `self.UpdateColour` (delegate `UpdateColour_Event`)))))

(event `UpdateColour_Event` :!signature `self.UpdateColour`
  (params (Colour :type "LinearColor Structure"))
  (`MaterialInstanceDynamic.SetVectorParameterValue` (`self.Material`) "EmissiveColour" Colour))

(fn `AddOutlineInsetVertPair`
  (params (OutlineVert :type "Vector Structure (by ref)"))
  ;[1 1 1] Add outline vert
  (`KismetArrayLibrary.Array_Add` (`self.Vertices`) OutlineVert)
  ;[1 1 1] Add calculated inset vert
  (`KismetArrayLibrary.Array_Add` (`self.Vertices`) (- OutlineVert (* (`KismetMathLibrary.Normal` OutlineVert) (`KismetMathLibrary.Conv_IntToVector` (`self.OutlineStroke`))))))

(fn `UserConstructionScript`
  (locals (MirroredOutlineVerts :type "Array of Vector Structure"))
  (bind _returnvalue (`PrimitiveComponent.CreateDynamicMaterialInstance` (`self.ProceduralMesh`) 0 "/Game/ByteWars/Materials/M_NeonGlow.M_NeonGlow" "None"))
  (set `self.Material` _returnvalue)
  (`MaterialInstanceDynamic.SetVectorParameterValue` _returnvalue "EmissiveColour" (`self.Colour`))
  (`MaterialInstanceDynamic.SetScalarParameterValue` _returnvalue "Glow" (`self.Glow`))
  (`ProceduralMeshComponent.ClearMeshSection` (`self.ProceduralMesh`) 0)
  (`|ExecutionSequence`
    (:`then_0`
      (`KismetArrayLibrary.Array_Clear` (`self.Vertices`))
      (`KismetArrayLibrary.Array_Clear` (`self.Triangles`))
      (for _array_element (`self.OutlineVertices`)
        (`KismetArrayLibrary.Array_Add` (`local.MirroredOutlineVerts`) _array_element))
      (bind (_arrayindex _arrayelement) (`/Engine/EditorBlueprintResources/StandardMacros.ReverseForEachLoop` (`self.OutlineVertices`))
        (:`LoopBody`
          (if (!= _arrayindex (- (`KismetArrayLibrary.Array_Length` (`self.OutlineVertices`)) 1))
            (`KismetArrayLibrary.Array_Add` (`local.MirroredOutlineVerts`) (`KismetMathLibrary.MirrorVectorByNormal` _arrayelement (1.0 0.0 0.0)))))
        (:`Completed`
          (for _array_element_2 (`local.MirroredOutlineVerts`)
            (`self.AddOutlineInsetVertPair` _array_element_2))
          (for (_ _array_index) (`local.MirroredOutlineVerts`)
            (for _array_element_3 (`self.TriStripPattern`)
              (`KismetArrayLibrary.Array_Add` (`self.Triangles`) (+ _array_element_3 (* _array_index 2))))))))
    (:`then_1`
      (`ProceduralMeshComponent.CreateMeshSection_LinearColor` :`self` (`self.ProceduralMesh`) :`Vertices` (`self.Vertices`) :`Triangles` (`self.Triangles`)))))