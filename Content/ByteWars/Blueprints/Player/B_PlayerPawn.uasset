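; Player pawn for ByteWars that fires one missile at a time, built on a procedural mesh set up at construction.
; Firing spawns a power-scaled missile, launch effect and attached player-colored trail, fades older trails and increments the player state's missile count.
; Tick shows the HUD power bar briefly after input and destroys faded trails.
; Other events recolor the mesh and pulse the camera background, skipping dedicated servers.
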(event `FireMissile_Event`
  (bind _rotation (.rotation (`self.GetTransform`)))
  ;[0 0 0] Fire missile
  (if (not (`KismetSystemLibrary.IsValid` (`self.FiredMissile`)))
    (`|ExecutionSequence`
      (:`then_0`
        ;;[0 0 0] Calculate where to spawn actors
        (set `self.FxSpawnTransform` (`KismetMathLibrary.MakeTransform` (+ (* (`KismetMathLibrary.GetRightVector` _rotation) 90.0) (.location (`self.GetTransform`))) _rotation)))
      (:`then_1`
        ;;[0 0 0] Spawn missile actor
        (bind _returnvalue (`|SpawnActorFromClass` "/Game/ByteWars/Blueprints/Missiles/B_Missile.B_Missile_C" (`self.FxSpawnTransform`) "Undefined" "OverrideRootScale" null (`KismetMathLibrary.MapRangeClamped` (`self.FirePowerLevel`) 0.0 1.0 (`self.MinMissileSpeed`) (`self.MaxMissileSpeed`)) self))
        (bind _output_get (set `self.FiredMissile` _returnvalue))
        (`/Game/ByteWars/Blueprints/Missiles/B_Missile.UpdateColor` _output_get (`AccelByteWarsProceduralMeshComponent.Color` (`self.AccelByteWarsProceduralMesh`)))
        (set `self.ShowPowerLevelUITimer` 0.0))
      (:`then_2`
        ;;[0 0 0] Fire missile fx
        (`|SpawnActorFromClass` "/Game/ByteWars/Blueprints/Ships/B_FireMissile.B_FireMissile_C" (`self.FxSpawnTransform`) "Undefined" "OverrideRootScale" null null))
      (:`then_3`
        ;;[0 0 0] Add missile to player state
        (bind _asb_in_game_player_state (cast `/Game/ByteWars/Blueprints/Player/B_InGamePlayerState` (`self.PlayerState`)))
        (set `/Game/ByteWars/Blueprints/Player/B_InGamePlayerState.NumMissilesFired` (+ (`/Game/ByteWars/Blueprints/Player/B_InGamePlayerState.NumMissilesFired` _asb_in_game_player_state) 1) _asb_in_game_player_state))
      (:`then_4`
        ;;[0 0 0] Missile trail
        ;;;[0 0 0] Start fade out on existing trails when new missile is fired
        (for _array_element (`self.MissileTrail`)
          (`/Game/ByteWars/Blueprints/Missiles/B_MissileTrail.TriggerFadeOut` _array_element))
        ;;;[0 0 0] Create missile trail, piggy back missile  and set colour to player
        (bind _returnvalue_2 (`|SpawnActorFromClass` "/Game/ByteWars/Blueprints/Missiles/B_MissileTrail.B_MissileTrail_C" (`self.FxSpawnTransform`) "Undefined" "OverrideRootScale" null null))
        (`KismetArrayLibrary.Array_Add` (`self.MissileTrail`) _returnvalue_2)
        (`self.K2_AttachToActor` _returnvalue_2 (`self.FiredMissile`) "None" "SnapToTarget" "SnapToTarget" "KeepRelative" true)
        (`/Game/ByteWars/Blueprints/Missiles/B_MissileTrail.UpdateColour` _returnvalue_2 (`AccelByteWarsProceduralMeshComponent.Color` (`self.AccelByteWarsProceduralMesh`)))))))

(event `self.ReceiveTick`
  (params (DeltaSeconds :type "Float (single-precision)"))
  (bind _showpowerleveluitimer (`self.ShowPowerLevelUITimer`))
  (bind _missiletrail (`self.MissileTrail`))
  ;[0 0 0] Event Tick sequence
  (`|ExecutionSequence`
    (:`then_0`
      ;;[0 0 0] Update PowerBar UI
      (bind _asplayer_controller (cast `PlayerController` (`self.GetController`)))
      (bind _asb_hud (cast `/Game/ByteWars/UI/HUD/B_HUD` (`PlayerController.GetHUD` _asplayer_controller)))
      (if (> _showpowerleveluitimer 0.0)
        (set `self.ShowPowerLevelUITimer` (`KismetMathLibrary.FClamp` (- _showpowerleveluitimer (`GameplayStatics.GetWorldDeltaSeconds`)) 0.0 100.0))
        (bind _powerbarui (`/Game/ByteWars/UI/HUD/B_HUD.PowerBarUI` _asb_hud))
        (`Widget.SetVisibility` _powerbarui "Visible")
        (else
          (`Widget.SetVisibility` _powerbarui "Hidden"))))
    (:`then_1`
      ;;[0 0 0] Remove faded out trails
      (bind (_arrayindex _arrayelement) (`/Engine/EditorBlueprintResources/StandardMacros.ReverseForEachLoop` _missiletrail)
        (:`LoopBody`
          (bind _isfadedout (`/Game/ByteWars/Blueprints/Missiles/B_MissileTrail.IsFadedOut` _arrayelement))
          (if _isfadedout
            (`self.K2_DestroyActor` _arrayelement)
            (`KismetArrayLibrary.Array_Remove` _missiletrail _arrayindex)))))))

(event `OnPlayerInputThisFrame_Event`
  ;[0 0 0] Events
  ;;[0 0 0] OnPlayerInputThisFrame
  (set `self.ShowPowerLevelUITimer` 1.0))

(event `UpdateColour_Event`
  (params (Colour :type "LinearColor Structure (by ref)"))
  ;[0 0 0] Events
  ;;[0 0 0] UpdateColor
  (`AccelByteWarsProceduralMeshComponent.UpdateColor` (`self.AccelByteWarsProceduralMesh`) Colour))

(event `PulseCameraBackground`
  ;[0 0 0] Events
  ;;[0 0 0] Pulse Camera background
  (if (not (`KismetSystemLibrary.IsDedicatedServer`))
    (bind _returnvalue (`GameplayStatics.GetActorOfClass` "/Game/ByteWars/Blueprints/Cameras/B_InGameCamera.B_InGameCamera_C"))
    (`/Game/ByteWars/Blueprints/Cameras/B_InGameCamera.PulseBackgroundEvent` _returnvalue)))

(fn `UserConstructionScript`
  (`AccelByteWarsProceduralMeshComponent.MeshSetup` (`self.AccelByteWarsProceduralMesh`)))