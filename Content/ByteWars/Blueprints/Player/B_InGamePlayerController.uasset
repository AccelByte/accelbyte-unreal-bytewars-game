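; B_InGamePlayerController is the in-match player controller for ByteWars, turning Enhanced Input actions into ship and UI commands.
; On BeginPlay it waits briefly, then for local players adds global and in-game mapping contexts and switches the view to the top-down B_InGameCamera.
; Input handles power, rotation, firing, power-ups, ship labels, help and session chat.
; Mouse capture is re-evaluated every tick and on input-method changes.
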(event `EnhancedInput|/Game/ByteWars/Blueprints/Input/InputActions/IA_AdjustPower`
  (params (ActionValue :type "Float (double-precision)") (ElapsedSeconds :type "Float (double-precision)") (TriggeredSeconds :type "Float (double-precision)") (InputAction :type "InputAction Object Reference" :default "/Game/ByteWars/Blueprints/Input/InputActions/IA_AdjustPower.IA_AdjustPower"))
  ;[0 0 0] Adjust Fire Power input listener
  (:`Started`
    (`self.AdjustPower` ActionValue :!label _label))
  (:`Completed`
    (goto _label)))

(event `EnhancedInput|/Game/ByteWars/Blueprints/Input/InputActions/IA_FireMissile`
  (params (ActionValue :type Boolean) (ElapsedSeconds :type "Float (double-precision)") (TriggeredSeconds :type "Float (double-precision)") (InputAction :type "InputAction Object Reference" :default "/Game/ByteWars/Blueprints/Input/InputActions/IA_FireMissile.IA_FireMissile"))
  ;[0 0 0] Fire missile input listener
  (:`Completed`
    (`self.FireMissile`)))

(event `self.ReceiveTick`
  (params (DeltaSeconds :type "Float (single-precision)"))
  ;[0 0 0] Tick sequence
  (`self.ToggleMouseCapture`))

(event `self.ReceiveBeginPlay`
  (bind _returnvalue (subsystem `CommonInputSubsystem`))
  (bind _returnvalue_2 (pcsubsystem `EnhancedInputLocalPlayerSubsystem` self))
  ;[0 0 0] BeginPlay sequence
  (`KismetSystemLibrary.Delay` 0.2)
  (if (`self.IsLocalPlayerController`)
    (`EnhancedInputSubsystemInterface.AddMappingContext` _returnvalue_2 "/Game/ByteWars/Blueprints/Input/InputMapping/IM_GlobalDefault.IM_GlobalDefault" 100 (struct))
    (`EnhancedInputSubsystemInterface.AddMappingContext` _returnvalue_2 "/Game/ByteWars/Blueprints/Input/InputMapping/IM_InGameDefault.IM_InGameDefault" 0 (struct))
    (`WidgetBlueprintLibrary.SetInputMode_GameOnly` self)
    (`self.EnableInput` self null)
    ;;[0 0 0] Use top down camera
    (bind _returnvalue_3 (`GameplayStatics.GetActorOfClass` "/Game/ByteWars/Blueprints/Cameras/B_InGameCamera.B_InGameCamera_C"))
    (`self.SetViewTargetWithBlend` _returnvalue_3)
    (`/Engine/EditorBlueprintResources/StandardMacros.IsValid` _returnvalue ; Check if input is valid or not
      (:`Is Valid`
        (add `CommonInputSubsystem.OnInputMethodChanged` _returnvalue (delegate `OnInputMethodChanged`))))))

(event `OnInputMethodChanged`
  (params (bNewInputType :type "ECommonInputType Enum" :default "MouseAndKeyboard"))
  ;[0 0 0] BeginPlay sequence
  (`self.ToggleMouseCapture`))

(event `EnhancedInput|/Game/ByteWars/Blueprints/Input/InputActions/IA_RotateShip_Clockwise`
  (params (ActionValue :type "Float (double-precision)") (ElapsedSeconds :type "Float (double-precision)") (TriggeredSeconds :type "Float (double-precision)") (InputAction :type "InputAction Object Reference" :default "/Game/ByteWars/Blueprints/Input/InputActions/IA_RotateShip_Clockwise.IA_RotateShip_Clockwise"))
  ;[0 0 0] RotateShip
  (:`Triggered`
    (`self.RotateShip` ActionValue :!label _label_2))
  (:`Ongoing`
    (goto _label_2))
  (:`Completed`
    (goto _label_2)))

(event `EnhancedInput|/Game/ByteWars/Blueprints/Input/InputActions/IA_RotateShip_CounterClockwise`
  (params (ActionValue :type "Float (double-precision)") (ElapsedSeconds :type "Float (double-precision)") (TriggeredSeconds :type "Float (double-precision)") (InputAction :type "InputAction Object Reference" :default "/Game/ByteWars/Blueprints/Input/InputActions/IA_RotateShip_CounterClockwise.IA_RotateShip_CounterClockwise"))
  ;[0 0 0] RotateShip
  (:`Triggered`
    (`self.RotateShip` ActionValue :!label _label_3))
  (:`Ongoing`
    (goto _label_3))
  (:`Completed`
    (goto _label_3)))

(event `EnhancedInput|/Game/ByteWars/Blueprints/Input/InputActions/IA_UsePowerUp`
  (params (ActionValue :type Boolean) (ElapsedSeconds :type "Float (double-precision)") (TriggeredSeconds :type "Float (double-precision)") (InputAction :type "InputAction Object Reference" :default "/Game/ByteWars/Blueprints/Input/InputActions/IA_UsePowerUp.IA_UsePowerUp"))
  ;[0 0 0] Activate Power Up
  (:`Completed`
    (`self.UsePowerUp`)))

(event `EnhancedInput|/Game/ByteWars/Blueprints/Input/InputActions/IA_OpenDevHelp`
  (params (ActionValue :type Boolean) (ElapsedSeconds :type "Float (double-precision)") (TriggeredSeconds :type "Float (double-precision)") (InputAction :type "InputAction Object Reference" :default "/Game/ByteWars/Blueprints/Input/InputActions/IA_OpenDevHelp.IA_OpenDevHelp"))
  ;[0 0 0] Open DevHelp / FTUE
  (:`Completed`
    (bind _asaccel_byte_wars_game_instance (cast `AccelByteWarsGameInstance` (`GameplayStatics.GetGameInstance`)))
    (`AccelByteWarsGameInstance.OpenFTUEMenu` _asaccel_byte_wars_game_instance)))

(event `EnhancedInput|/Game/ByteWars/Blueprints/Input/InputActions/IA_OpenGameSessionChat`
  (params (ActionValue :type Boolean) (ElapsedSeconds :type "Float (double-precision)") (TriggeredSeconds :type "Float (double-precision)") (InputAction :type "InputAction Object Reference" :default "/Game/ByteWars/Blueprints/Input/InputActions/IA_OpenGameSessionChat.IA_OpenGameSessionChat"))
  ;[0 0 0] Open Game Session Chat
  (:`Completed`
    (bind _asaccel_byte_wars_game_instance (cast `AccelByteWarsGameInstance` (`GameplayStatics.GetGameInstance`)))
    (`AccelByteWarsBaseUI.PushWidgetToStack` (`AccelByteWarsGameInstance.GetBaseUIWidget` _asaccel_byte_wars_game_instance true) "InGameMenu" "/Game/TutorialModules/Social/SessionChat/UI/W_SessionChat.W_SessionChat_C")))

(event `EnhancedInput|/Game/ByteWars/Blueprints/Input/InputActions/IA_ToggleShipLabel`
  (params (ActionValue :type Boolean) (ElapsedSeconds :type "Float (double-precision)") (TriggeredSeconds :type "Float (double-precision)") (InputAction :type "InputAction Object Reference" :default "/Game/ByteWars/Blueprints/Input/InputActions/IA_ToggleShipLabel.IA_ToggleShipLabel"))
  ;[0 0 0] Toggle Ship Labels
  (:`Completed`
    (bind _outactors (`GameplayStatics.GetAllActorsOfClass` "/Game/ByteWars/Blueprints/Player/ABPawn.ABPawn_C"))
    (for _array_element _outactors
      (`/Engine/EditorBlueprintResources/StandardMacros.IsValid` _array_element
        (:`Is Valid`
          (`AccelByteWarsPlayerPawn.ToggleShipLabel` _array_element))))))

(fn `UserConstructionScript`)